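; BP_Water is a water actor whose height follows the shared water level held in BP_MainGS, the game state.
; On BeginPlay it passes its starting Z and its FullZ value to the game state to initialize the water values.
; Every tick, only on authority, it sets its Z to the game state's WaterHeight, keeping X and Y unchanged.
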(event EventBeginPlay
  ;[1 1 1] 초기화
  (bind _asbp_main_gs (Utilities|Casting|CastToBP_MainGS (Game|GetGameState)))
  (Default|InitWaterValues _asbp_main_gs (.z (Transformation|GetActorLocation)) (Variables|Default|GetFullZ)))

(event EventTick
  (params (DeltaSeconds :type Float%20%28single-precision%29))
  (bind _returnvalue (Transformation|GetActorLocation))
  ;[1 1 1] Tick
  (Networking|SwitchHasAuthority
    (:Authority
      (bind _asbp_main_gs (Utilities|Casting|CastToBP_MainGS (Game|GetGameState)))
      (Transformation|SetActorLocation (Math|Vector|MakeVector (.x _returnvalue) (.y _returnvalue) (Variables|/Game/Blueprints/System/Main/BP_MainGS.BP_MainGS_C|GetWaterHeight _asbp_main_gs)) false false))))

(fn ConstructionScript)