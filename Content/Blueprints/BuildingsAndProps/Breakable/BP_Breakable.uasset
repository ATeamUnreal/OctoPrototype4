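; Breakable prop that vanishes with an explosion sound when a motion controller or SN projectile overlaps its box.
; On authority, Destruction disables box collision, hides the mesh and destroys the actor after a short delay.
; The sound is relayed through ServerSound to MulticastSound at the actor's location.
; AnyDamage is empty, and the destructible-mesh debris spawn (SpawnDM) is disconnected, so no debris appears.
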(event OnComponentBeginOverlap(Box)
  (params (OverlappedComponent :type Primitive%20Component%20Object%20Reference) (OtherActor :type Actor%20Object%20Reference) (OtherComp :type Primitive%20Component%20Object%20Reference) (OtherBodyIndex :type Integer) (bFromSweep :type Boolean) (SweepResult :type Hit%20Result%20Structure%20%28by%20ref%29))
  ;[1 1 1] 데미지를 받으면 부서짐
  (Utilities|Casting|CastToBP_MotionControllerMain OtherActor
    (:then
      _)
    (:CastFailed
      (Utilities|Casting|CastToBP_Projectile_SN OtherActor)))
  (Networking|SwitchHasAuthority
    (:Authority
      (if (not (Utilities|Enum|Equal(Enum) (Collision|GetCollisionEnabled (Variables|Default|GetBox)) "NoCollision"))
        (CallFunction|Destruction)))))

(event Custom|Destruction
  ;[1 1 1] 코멘트
  (Collision|SetCollisionEnabled (Variables|Default|GetBox) "NoCollision")
  (Rendering|SetVisibility (Variables|Default|GetStaticMesh) false false)
  (CallFunction|PlaySound)
  (Utilities|FlowControl|Delay 2.0)
  (Actor|DestroyActor))

(event Custom|MulticastSound
  (params (SoundLocation :type Vector))
  ;[1 1 1] 코멘트
  (Audio|SpawnSoundatLocation "/Game/Ultimate_SFX_Bundle/Warfare_SFX_Bundle/Explosion_Sounds_Pro/Cues/Explosion_Gas_02_Cue.Explosion_Gas_02_Cue" SoundLocation "0, 0, 0" 1.0 1.0 0.0 0 0))

(event Custom|ServerSound
  (params (SoundLocation :type Vector))
  ;[1 1 1] 코멘트
  (CallFunction|MulticastSound SoundLocation))

(event Custom|PlaySound
  ;[1 1 1] 코멘트
  (CallFunction|ServerSound (Transformation|GetActorLocation)))

(event Custom|SpawnDM
  ;[1 1 1] 부서짐잔해표시
  (bind _returnvalue (Game|SpawnActorfromClass "/Game/Blueprints/BuildingsAndProps/Breakable/BP_Breakable_DM.BP_Breakable_DM_C" (Transformation|GetActorTransform) "AlwaysSpawn" 0 0))
  (Default|Destruction _returnvalue (Variables|Default|GetDMLifeTime) (Variables|Default|GetDestructibleMesh) (Transformation|GetWorldTransform (Variables|Default|GetStaticMesh)) (Variables|Default|GetImpulseStrength)))

(event Game|Damage|EventAnyDamage
  (params (Damage :type Float%20%28single-precision%29) (DamageType :type Damage%20Type%20Object%20Reference) (InstigatedBy :type Controller%20Object%20Reference) (DamageCauser :type Actor%20Object%20Reference)))

(fn ConstructionScript)