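; Main game state that tracks the hunters' respawn pool and drives the match's rising water.
; Respawn decrements refresh the hunter widget, also through a RepNotify, and tell BP_MainGM to end the game at zero.
; On authority, Tick raises blue water to its target height, waits, then raises dead water beyond it at speeds derived from set durations.
; Switching to the Playing state ends loading through the first player controller.
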(event Custom|DecreaseRespawnCount
  ;[1 1 1] 리스폰카운트 업데이트
  (Math|Integer|DecrementInt (Variables|Default|GetRespawnCount)
    (:%20%20
      ;;[1 1 1] 서버쪽에서의  UI업데이트
      (bind _asbp_main_pc (Utilities|Casting|CastToBP_MainPC (Game|GetPlayerController 0)))
      (Utilities|IsValid _asbp_main_pc
        (:Is%20Valid
          (Default|UpdateHunterMainWidgetServer _asbp_main_pc)
          (if (not (> (Variables|Default|GetRespawnCount) 0))
            (Variables|Default|SetRespawnCount 0)
            (bind _asbp_main_gm (Utilities|Casting|CastToBP_MainGM (Game|GetGameMode)))
            (Utilities|IsValid _asbp_main_gm
              (:Is%20Valid
                (Default|GameOver _asbp_main_gm false)))))))))

(event EventBeginPlay
  (CallFunction|InitRespawnCount))

(event EventTick
  (params (DeltaSeconds :type Float%20%28single-precision%29))
  ;[1 1 1] Tick
  (Networking|SwitchHasAuthority
    (:Authority
      (CallFunction|RiseWater DeltaSeconds)
      (CallFunction|CheckWaterState DeltaSeconds))))

(event EventDowhenCurrentGameStateChanged
  (if (Utilities|Enum|Equal(Enum) (Variables|Default|GetCurrentGameState) "Playing")
    (bind _asbp_main_pc (Utilities|Casting|CastToBP_MainPC (Game|GetPlayerController 0)))
    (Default|EndLoadingServer _asbp_main_pc)))

(fn ConstructionScript)

(fn InitRespawnCount
  (Variables|Default|SetRespawnCount (Variables|Default|GetMaxRespawnCount)))

(fn InitWaterValues
  (params (InitialZ :type Float%20%28single-precision%29) (FullZ :type Float%20%28single-precision%29))
  (Variables|Water|SetBlueWaterHeight InitialZ)
  (Variables|Water|SetWaterFinalZ FullZ)
  (Variables|Water|SetBlueWaterSpeed (/ (- (Variables|Water|GetWaterFinalZ) (Variables|Water|GetBlueWaterHeight)) (Variables|Water|GetBlueWaterTime)))
  (Variables|Water|SetAfterBlueWaterTime 0.0)
  (Variables|Water|SetIsBlueWaterRising true))

(fn Test
  (for _array_element (Variables|Default|GetPlayerArray)
    (bind _asbp_main_ps (Utilities|Casting|CastToBP_MainPS _array_element))
    (LocalVariables|SetdebugText (Utilities|String|Append (LocalVariables|GetdebugText) " " (Utilities|String|ToString(Float) (Variables|/Game/Blueprints/System/Main/BP_MainPS.BP_MainPS_C|GetCurrentHP _asbp_main_ps)))))
  (Development|PrintString (LocalVariables|GetdebugText)))

(fn OnRepRespawnCount
  (bind _asbp_main_pc (Utilities|Casting|CastToBP_MainPC (Game|GetPlayerController 0)))
  (Utilities|IsValid _asbp_main_pc
    (:Is%20Valid
      (Default|UpdateHunterMainWidgetServer _asbp_main_pc))))

(fn RiseWater
  (params (DeltaSeconds :type Float%20%28single-precision%29))
  ;[1 1 1] BlueWater
  (if (Variables|Water|GetIsBlueWaterRising)
    (Variables|Water|SetBlueWaterHeight (+ (Variables|Water|GetBlueWaterHeight) (* DeltaSeconds (Variables|Water|GetBlueWaterSpeed))))
    (if (> (Variables|Water|GetBlueWaterHeight) (Variables|Water|GetWaterFinalZ))
      (Variables|Water|SetIsBlueWaterRising false)
      (Development|PrintString "BlueWaterDone" true true "(R=0.000000,G=0.660000,B=1.000000,A=1.000000)" 1e+02))
    (else
      ;[1 1 1] DeadWater
      (if (Variables|Water|GetIsDeadWaterRising)
        (Variables|Water|SetDeadWaterHeight (+ (Variables|Water|GetDeadWaterHeight) (* DeltaSeconds (Variables|Water|GetDeadWaterSpeed))))
        (if (> (Variables|Water|GetDeadWaterHeight) (+ (Variables|Water|GetWaterFinalZ) 1.9e+03))
          (Variables|Water|SetIsDeadWaterRising false)
          (Development|PrintString "DeadWaterDone" true true "(R=0.000000,G=0.660000,B=1.000000,A=1.000000)" 1e+02)
          (Variables|Water|SetRiseWaterDone true))))))

(fn CheckWaterState
  (params (DeltaSeconds :type Float%20%28single-precision%29))
  (if (not (Variables|Water|GetRiseWaterDone))
    (if (not (Variables|Water|GetIsBlueWaterRising))
      (if (not (Variables|Water|GetIsDeadWaterRising))
        (Variables|Water|SetAfterBlueWaterTime (+ DeltaSeconds (Variables|Water|GetAfterBlueWaterTime)))
        (if (> (Variables|Water|GetAfterBlueWaterTime) (Variables|Water|GetDeadWaterStartTime))
          (Variables|Water|SetIsDeadWaterRising true))))))

(fn InitDeadWaterValues
  (params (InitialZ :type Float%20%28single-precision%29))
  (bind _output_get (Variables|Water|SetDeadWaterHeight InitialZ))
  (Variables|Water|SetDeadWaterSpeed (/ (- (Variables|Water|GetWaterFinalZ) _output_get) (Variables|Water|GetDeadWaterTime))))